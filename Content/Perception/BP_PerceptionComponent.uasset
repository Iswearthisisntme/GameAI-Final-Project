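; BP_PerceptionComponent is a perception component that visualizes the states of the targets tracked for its owning pawn.
; When Debug is enabled, Tick calls DrawTargetDebug, which loops over the cached target states and draws a debug line from the pawn for each.
; Line color reflects Unknown, Immediate or Hidden state.
; Immediate and Hidden lines end at the cached position, while Unknown lines end at the first player's pawn.
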(event EventBeginPlay)

(event EventTick
  (params (DeltaSeconds :type Float%20%28single-precision%29))
  (if (Variables|Default|GetDebug)
    (CallFunction|DrawTargetDebug)))

(fn DrawTargetDebug
  (bind (_targetcachesout _targetdatasout) (Class|GAPerceptionComponent|GetAllTargetStates false))
  (LocalVariables|SetTargetCaches _targetcachesout)
  (LocalVariables|SetTargetDatas _targetdatasout)
  (for _array_element (LocalVariables|GetTargetCaches)
    (Utilities|FlowControl|Sequence
      (:then_0
        (switch Utilities|FlowControl|Switch|SwitchonETargetState (.State (Utilities|Struct|BreakTargetCache _array_element))
          (:GATS_Unknown
            (LocalVariables|SetColor "(R=0.313542,G=0.313542,B=0.313542,A=1.000000)")
            (LocalVariables|SetTargetPoint (Transformation|GetActorLocation (Game|Player|GetPlayerPawn 0))))
          (:GATS_Immediate
            (LocalVariables|SetColor "(R=0.059217,G=1.000000,B=0.000000,A=1.000000)")
            (LocalVariables|SetTargetPoint (.Position (Utilities|Struct|BreakTargetCache _array_element))))
          (:GATS_Hidden
            (LocalVariables|SetColor "(R=0.013500,G=0.091829,B=1.000000,A=1.000000)")
            (LocalVariables|SetTargetPoint (.Position (Utilities|Struct|BreakTargetCache _array_element))))))
      (:then_1
        (Rendering|Debug|DrawDebugLine (Transformation|GetActorLocation (Class|GAPerceptionComponent|GetOwnerPawn)) (LocalVariables|GetTargetPoint) (LocalVariables|GetColor) 0.0 0.0)))))